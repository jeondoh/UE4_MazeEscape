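; Health pickup actor for the maze game that restores health to the player who touches it.
; Sphere overlap with a BP_MazePlayer adds the healing amount to Health, capped at MaxHealth, then plays a pickup sound and destroys the actor.
; An optional Rotate flag spins the pickup around its yaw axis on Tick at RotateSpeed, scaled by delta time.
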(event `self.ReceiveBeginPlay`)

(event `self.ReceiveTick`
  (params (DeltaSeconds :type "Float (single-precision)"))
  (bind (_returnvalue_roll _returnvalue_pitch _returnvalue_yaw) (`KismetMathLibrary.BreakRotator` (`self.K2_GetActorRotation`)))
  (if (`self.bRotate`)
    (`self.K2_SetActorRotation` (`KismetMathLibrary.MakeRotator` _returnvalue_roll _returnvalue_pitch (+ _returnvalue_yaw (* DeltaSeconds (.yaw (`KismetMathLibrary.MakeRotator` 0.0 0.0 (`self.RotateSpeed`)))))))))

(event `self.Sphere.OnComponentBeginOverlap`
  (params (OverlappedComponent :type "PrimitiveComponent Object Reference") (OtherActor :type "Actor Object Reference") (OtherComp :type "PrimitiveComponent Object Reference") (OtherBodyIndex :type Integer) (bFromSweep :type Boolean) (SweepResult :type "HitResult Structure (by ref)"))
  (bind _asbp_maze_player (cast `/Game/00_MazeDev/Character/Blueprints/BP_MazePlayer` OtherActor))
  (bind _returnvalue (+ (`self.HealingAmount`) (`MazePlayer.Health` _asbp_maze_player)))
  (bind _maxhealth (`MazePlayer.MaxHealth` _asbp_maze_player))
  (if (> _returnvalue _maxhealth)
    (set `MazePlayer.Health` _maxhealth _asbp_maze_player)
    (else
      (set `MazePlayer.Health` _returnvalue _asbp_maze_player)))
  (`GameplayStatics.PlaySoundAtLocation` "/Game/00_MazeDev/Sounds/Pickup/Pickup_Health_Cue.Pickup_Health_Cue" (`self.K2_GetActorLocation`) (struct) 1.0 1.0 0.0 null null null)
  (`self.K2_DestroyActor`))

(fn `UserConstructionScript`)