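; BP_Boss is the maze game's boss enemy, with a screen health bar and a game-clear screen on defeat.
; Overlapping AgroSphere caches the BP_MazePlayer and toggles health bar visibility as the player enters or leaves.
; Tick copies health to that player and, at zero, waits briefly, stops ticking and shows Widget_GameClear.
; ShowHitNumber spawns animated damage widgets at the projected hit location, flagging headshots.
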(event `self.ReceiveBeginPlay`
  (`parent.ReceiveBeginPlay`)
  (bind _returnvalue (`|CreateWidget` "/Game/00_MazeDev/HUD/BP_Boss_HealthBar.BP_Boss_HealthBar_C" (`GameplayStatics.GetPlayerController` 0)))
  (bind _output_get (set `self.BossHealthBar` _returnvalue))
  (`UserWidget.AddToViewport` _output_get 0)
  (`Widget.SetVisibility` _output_get "Hidden"))

(event `self.ShowHitNumber`
  (params (Damage :type Integer) (HitLocation :type "Vector Structure") (bHeadShot :type Boolean))
  (bind _returnvalue (`|CreateWidget` "/Game/00_MazeDev/HUD/BP_HitNUmber.BP_HitNumber_C"))
  (`UserWidget.AddToViewport` _returnvalue 0)
  (`UserWidget.SetPositionInViewport` _returnvalue (`GameplayStatics.ProjectWorldToScreen` (`GameplayStatics.GetPlayerController` 0) HitLocation) true)
  (`self.StoreHitNumber` _returnvalue HitLocation)
  (set `/Game/00_MazeDev/HUD/BP_HitNUmber.HitText` (`KismetTextLibrary.Conv_IntToText` Damage) _returnvalue)
  (set `/Game/00_MazeDev/HUD/BP_HitNUmber.HeadShot` bHeadShot _returnvalue)
  (`UserWidget.PlayAnimation` _returnvalue (`/Game/00_MazeDev/HUD/BP_HitNUmber.HitNumberAnimation` _returnvalue) 0.0 1 "Forward" 1.0 false))

(event `self.ReceiveTick`
  (params (DeltaSeconds :type "Float (single-precision)"))
  (bind _mazeplayer (`self.MazePlayer`))
  (`/Engine/EditorBlueprintResources/StandardMacros.IsValid` _mazeplayer
    (:`Is Valid`
      (set `MazePlayer.BossHealth` (`self.Health`) _mazeplayer)
      (set `MazePlayer.BossMaxHealth` (`self.MaxHealth`) _mazeplayer)
      (if (<= (`MazePlayer.BossHealth` _mazeplayer) 0.0)
        (`KismetSystemLibrary.Delay` 1.0)
        (`self.SetActorTickEnabled` false)
        (bind _returnvalue (`|CreateWidget` "/Game/Megascans/Blueprints/UI/Intro_Outro/Widget_GameClear.Widget_GameClear_C"))
        (`UserWidget.AddToViewport` _returnvalue 0)))))

(event `self.AgroSphere.OnComponentBeginOverlap`
  (params (OverlappedComponent :type "PrimitiveComponent Object Reference") (OtherActor :type "Actor Object Reference") (OtherComp :type "PrimitiveComponent Object Reference") (OtherBodyIndex :type Integer) (bFromSweep :type Boolean) (SweepResult :type "HitResult Structure (by ref)"))
  (bind _asbp_maze_player (cast `/Game/00_MazeDev/Character/Blueprints/BP_MazePlayer` OtherActor))
  (bind _output_get (set `self.MazePlayer` _asbp_maze_player))
  (set `MazePlayer.isBossHealthVisible` true _output_get)
  (`Widget.SetVisibility` (`self.BossHealthBar`) "Visible"))

(event `self.AgroSphere.OnComponentEndOverlap`
  (params (OverlappedComponent :type "PrimitiveComponent Object Reference") (OtherActor :type "Actor Object Reference") (OtherComp :type "PrimitiveComponent Object Reference") (OtherBodyIndex :type Integer))
  (bind _asbp_maze_player (cast `/Game/00_MazeDev/Character/Blueprints/BP_MazePlayer` OtherActor))
  (set `MazePlayer.isBossHealthVisible` false _asbp_maze_player)
  (`Widget.SetVisibility` (`self.BossHealthBar`) "Hidden"))

(fn `UserConstructionScript`)