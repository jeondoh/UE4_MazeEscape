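; Anim notify that plays surface-dependent footstep effects for the maze player character.
; It casts the mesh owner to BP_MazePlayer, reads its surface type, and picks a sound cue and Niagara system for metal, stone, tile, grass or water.
; It spawns the particles at the notify's bone socket and plays the sound there only when ShouldPlaySound is set.
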(fn `Received_Notify`
  (params (MeshComp :type "SkeletalMeshComponent Object Reference") (Animation :type "AnimSequenceBase Object Reference"))
  (returns (ReturnValue :type Boolean))
  (locals (FootStepSound :type "SoundBase Object Reference" :default "SoundCue'/Game/00_MazeDev/Sounds/FootSteps/FootStep_Tile_Cue.FootStep_Tile_Cue'") (FootStepNiagaraSystem :type "NiagaraSystem Object Reference" :default "NiagaraSystem'/Game/A_Surface_Footstep/Niagara_FX/ParticleSystems/PSN_General2_Surface.PSN_General2_Surface'"))
  (bind _returnvalue (`SceneComponent.GetSocketLocation` MeshComp (`self.BoneName`)))
  (bind _asbp_maze_player (cast `/Game/00_MazeDev/Character/Blueprints/BP_MazePlayer` (`ActorComponent.GetOwner` MeshComp)))
  (bind _returnvalue_2 (`MazePlayer.GetSurfaceType` _asbp_maze_player))
  (switch `EPhysicalSurface` _returnvalue_2
    (:`SurfaceType_Default`
      _)
    (:`SurfaceType1`
      (set `local.FootStepSound` "/Game/00_MazeDev/Sounds/FootSteps/FootStep_Metal_Cue.FootStep_Metal_Cue")
      (set `local.FootStepNiagaraSystem` "/Game/A_Surface_Footstep/Niagara_FX/ParticleSystems/PSN_General1_Surface.PSN_General1_Surface"))
    (:`SurfaceType2`
      (set `local.FootStepSound` "/Game/00_MazeDev/Sounds/FootSteps/FootStep_Stone_Cue.FootStep_Stone_Cue")
      (set `local.FootStepNiagaraSystem` "/Game/A_Surface_Footstep/Niagara_FX/ParticleSystems/PSN_Dirt_Surface.PSN_Dirt_Surface"))
    (:`SurfaceType3`
      (set `local.FootStepSound` "/Game/00_MazeDev/Sounds/FootSteps/FootStep_Tile_Cue.FootStep_Tile_Cue")
      (set `local.FootStepNiagaraSystem` "/Game/A_Surface_Footstep/Niagara_FX/ParticleSystems/PSN_General1_Surface.PSN_General1_Surface"))
    (:`SurfaceType4`
      (set `local.FootStepSound` "/Game/00_MazeDev/Sounds/FootSteps/FootStep_Grass_Cue.FootStep_Grass_Cue")
      (set `local.FootStepNiagaraSystem` "/Game/A_Surface_Footstep/Niagara_FX/ParticleSystems/PSN_Grass_Surface.PSN_Grass_Surface"))
    (:`SurfaceType5`
      (set `local.FootStepSound` "/Game/00_MazeDev/Sounds/FootSteps/FootStep_Water_Cue.FootStep_Water_Cue")
      (set `local.FootStepNiagaraSystem` "/Game/A_Surface_Footstep/Niagara_FX/ParticleSystems/PSN_WaterHeavy_Surface.PSN_WaterHeavy_Surface")))
  (if (`self.bShouldPlaySound`)
    (`GameplayStatics.PlaySoundAtLocation` (`local.FootStepSound`) _returnvalue (struct) 1.0 1.0 0.0 null null null))
  (`NiagaraFunctionLibrary.SpawnSystemAtLocation` (`local.FootStepNiagaraSystem`) _returnvalue)
  (return true))