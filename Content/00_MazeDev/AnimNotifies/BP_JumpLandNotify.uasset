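; Animation notify that plays a surface-specific landing sound when BP_MazePlayer lands from a jump.
; It casts the mesh owner to BP_MazePlayer, reads its surface type and selects a metal, stone, tile, grass or water cue, with tile as the fallback.
; The cue plays through PlaySoundAtLocation at a fixed world origin rather than the player's position.
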(fn `Received_Notify`
  (params (MeshComp :type "SkeletalMeshComponent Object Reference") (Animation :type "AnimSequenceBase Object Reference"))
  (returns (ReturnValue :type Boolean))
  (locals (LandingSound :type "SoundBase Object Reference"))
  (bind _asbp_maze_player (cast `/Game/00_MazeDev/Character/Blueprints/BP_MazePlayer` (`ActorComponent.GetOwner` MeshComp)))
  (bind _returnvalue (`MazePlayer.GetSurfaceType` _asbp_maze_player))
  (switch `EPhysicalSurface` _returnvalue
    (:`SurfaceType_Default`
      (set `local.LandingSound` "/Game/00_MazeDev/Sounds/FootSteps/FootStep_LandTile_Cue.FootStep_LandTile_Cue"))
    (:`SurfaceType1`
      (set `local.LandingSound` "/Game/00_MazeDev/Sounds/FootSteps/FootStep_LandMetal_Cue.FootStep_LandMetal_Cue"))
    (:`SurfaceType2`
      (set `local.LandingSound` "/Game/00_MazeDev/Sounds/FootSteps/FootStep_Stone_Cue.FootStep_Stone_Cue"))
    (:`SurfaceType3`
      (set `local.LandingSound` "/Game/00_MazeDev/Sounds/FootSteps/FootStep_LandTile_Cue.FootStep_LandTile_Cue"))
    (:`SurfaceType4`
      (set `local.LandingSound` "/Game/00_MazeDev/Sounds/FootSteps/FootStep_LandGrass_Cue.FootStep_LandGrass_Cue"))
    (:`SurfaceType5`
      (set `local.LandingSound` "/Game/00_MazeDev/Sounds/FootSteps/FootStep_LandWater_Cue.FootStep_LandWater_Cue")))
  (`GameplayStatics.PlaySoundAtLocation` (`local.LandingSound`) (0.0 0.0 0.0) (struct) 1.0 1.0 0.0 null null null)
  (return true))