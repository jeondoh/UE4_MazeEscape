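; HUD Blueprint that draws the maze player's dynamic crosshair at screen center.
; Each DrawHUD uses the cached BP_MazePlayer, lazily casting the player pawn when that reference is invalid.
; Five crosshair textures come from the equipped weapon, with top, bottom, left and right pushed outward by the player's spread multiplier times a maximum spread.
; BeginPlay only performs an empty validity check, and a second cast chain is never run.
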(event `self.ReceiveBeginPlay`
  ;[1 1 1] MazePlayer 형변환
  (`/Engine/EditorBlueprintResources/StandardMacros.IsValid` (`self.MazePlayer`)))

(event `self.ReceiveDrawHUD`
  (params (SizeX :type Integer) (SizeY :type Integer))
  (bind (_x _y) (`KismetMathLibrary.BreakVector2D` (`self.CrosshairBaseCenter`)))
  (bind (_x_2 _y_2) (`KismetMathLibrary.BreakVector2D` (`self.CrosshairBaseCenter`)))
  (bind (_x_3 _y_3) (`KismetMathLibrary.BreakVector2D` (`self.CrosshairBaseCenter`)))
  (bind (_x_4 _y_4) (`KismetMathLibrary.BreakVector2D` (`self.CrosshairBaseCenter`)))
  (bind (_x_5 _y_5) (`KismetMathLibrary.BreakVector2D` (`self.CrosshairBaseCenter`)))
  (bind (_x_6 _y_6) (`KismetMathLibrary.BreakVector2D` (`self.CrosshairLocation`)))
  ;[1 1 1] 화면 중앙 구하기
  (bind _output_get (set `self.Screen Center` (`KismetMathLibrary.MakeVector2D` (`KismetMathLibrary.Conv_IntToDouble` (/ SizeX 2)) (`KismetMathLibrary.Conv_IntToDouble` (/ SizeY 2)))))
  (set `self.CrosshairLocation` _output_get)
  (`/Engine/EditorBlueprintResources/StandardMacros.IsValid` (`self.MazePlayer`)
    (:`Is Valid`
      _)
    (:`Is Not Valid`
      (bind _asbp_maze_player (cast `/Game/00_MazeDev/Character/Blueprints/BP_MazePlayer` (`GameplayStatics.GetPlayerPawn` 0)))
      (set `self.MazePlayer` _asbp_maze_player)))
  (set `self.CrosshairSpreadMuliplier` (`MazePlayer.GetCrosshairSpreadMultiplier` (`self.MazePlayer`)))
  (set `self.CrosshairBaseCenter` (`KismetMathLibrary.MakeVector2D` (- _x_6 (`self.CrosshairHalfWidth`)) (- _y_6 (`self.CrosshairHalfHeight`))))
  ;[1 1 1] Crosshair 아래
  (`self.DrawTexture` (`Weapon.CrosshairsBottom` (`MazePlayer.EquippedWeapon` (`self.MazePlayer`))) _x_3 (+ _y_3 (* (`self.CrosshairSpreadMuliplier`) (`self.CrosshairSpreadMax`))) 64.0 64.0 0.0 0.0 1.0 1.0)
  ;[1 1 1] Crosshair 위
  (`self.DrawTexture` (`Weapon.CrosshairsTop` (`MazePlayer.EquippedWeapon` (`self.MazePlayer`))) _x_4 (- _y_4 (* (`self.CrosshairSpreadMuliplier`) (`self.CrosshairSpreadMax`))) 64.0 64.0 0.0 0.0 1.0 1.0)
  ;[1 1 1] Crosshair 왼쪽
  (`self.DrawTexture` (`Weapon.CrosshairsLeft` (`MazePlayer.EquippedWeapon` (`self.MazePlayer`))) (- _x (* (`self.CrosshairSpreadMuliplier`) (`self.CrosshairSpreadMax`))) _y 64.0 64.0 0.0 0.0 1.0 1.0)
  ;[1 1 1] Crosshair 오른쪽
  (`self.DrawTexture` (`Weapon.CrosshairsRight` (`MazePlayer.EquippedWeapon` (`self.MazePlayer`))) (+ (* (`self.CrosshairSpreadMuliplier`) (`self.CrosshairSpreadMax`)) _x_2) _y_2 64.0 64.0 0.0 0.0 1.0 1.0)
  (`self.DrawTexture` (`Weapon.CrosshairsMiddle` (`MazePlayer.EquippedWeapon` (`self.MazePlayer`))) _x_5 _y_5 64.0 64.0 0.0 0.0 1.0 1.0))

(fn `UserConstructionScript`)