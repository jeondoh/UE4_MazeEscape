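; A double sliding door Blueprint that opens when something enters its trigger box and closes when it leaves.
; Box begin overlap plays the Slide timeline, and end overlap reverses it.
; Each timeline update lerps the left and right door components' relative locations between stored current and new vectors.
; Overlaps are not filtered by actor, and movement is applied without sweep.
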(event `self.Box.OnComponentBeginOverlap`
  (params (OverlappedComponent :type "PrimitiveComponent Object Reference") (OtherActor :type "Actor Object Reference") (OtherComp :type "PrimitiveComponent Object Reference") (OtherBodyIndex :type Integer) (bFromSweep :type Boolean) (SweepResult :type "HitResult Structure (by ref)"))
  (bind (_direction `_새_트랙_0`) (`Timeline|Slide` :!label _label)
    (:`Update`
      (`SceneComponent.K2_SetRelativeLocation` (`self.RIGHT_SlideDoor`) (`KismetMathLibrary.VLerp` (`self.RIGHT_CurrentVector`) (`self.RIGHT_NewVector`) `_새_트랙_0`) false false)
      (`SceneComponent.K2_SetRelativeLocation` (`self.LEFT_SlideDoor`) (`KismetMathLibrary.VLerp` (`self.LEFT_CurrentVector`) (`self.LEFT_NewVector`) `_새_트랙_0`) false false))))

(event `self.Box.OnComponentEndOverlap`
  (params (OverlappedComponent :type "PrimitiveComponent Object Reference") (OtherActor :type "Actor Object Reference") (OtherComp :type "PrimitiveComponent Object Reference") (OtherBodyIndex :type Integer))
  (goto _label :!via `Reverse`))

(fn `UserConstructionScript`)